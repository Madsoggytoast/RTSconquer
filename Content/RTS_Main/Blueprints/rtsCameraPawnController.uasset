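; RTS player controller that drives the camera pawn, cursor interaction and grid-based placement.
; BeginPlay caches references, spawns construction manager and ghost building actors, then shows the main HUD and starts the game.
; Input moves, edge-scrolls, pans and zooms the camera, with keyboard speed scaled by zoom.
; A 250-unit snapped cursor trace moves the ghost and grid, places energy-costed decals in attack mode, or otherwise selects decals to show their widgets.
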(event `Spawn_building`
  (params (Class :type "Actor Class Reference") (SpawnTransform :type "Transform Structure") (Owner :type "Actor Object Reference"))
  ;[1 1 1] Spawn Building
  (`|SpawnActorFromClass` Class SpawnTransform "Undefined" "OverrideRootScale" Owner null))

(event `Toogle_widget`
  (params (Actor :type "Actor Object Reference") (NewHidden :type Boolean))
  ;[1 1 1] Show Widget
  (bind _asdecal_actor (cast `/Game/RTS_Main/Blueprints/Decal/Decal_actor` Actor))
  (`SceneComponent.SetHiddenInGame` (`/Game/RTS_Main/Blueprints/Decal/Decal_actor.Widget` _asdecal_actor) NewHidden false)
  (set `self.Targeted_decal` _asdecal_actor))

(event `Server_spawn`
  (params (SpawnTransform :type "Transform Structure") (Owner :type "Actor Object Reference") (Player_color :type "SlateColor Structure"))
  ;[1 1 1] Spawn decal
  (`|SpawnActorFromClass` "/Game/RTS_Main/Blueprints/Decal/Decal_actor.Decal_actor_C" SpawnTransform "Undefined" "OverrideRootScale" Owner Player_color null))

(event `Key|LeftMouseButton`
  (params (Key :type "Key Structure"))
  ;[1 1 1] Left Mouse Button
  (:`Pressed`
    (`self.Click_widget`)
    (if (`self.Attack Mode`)
      (bind (_newparam _returnvalue) (`self.Get_location`))
      (if (not _returnvalue)
        (bind _newparam_2 (`self.Have_energy?` 2))
        (if _newparam_2
          (`self.Server_spawn` (`KismetMathLibrary.MakeTransform` _newparam (struct) (2.5 2.22 2.5)) self (`self.Color chosen`))
          (`self.Change_energy` -2)))
      (else
        (bind (_newparam_3 _returnvalue_2 _hitactor) (`self.Get_location`))
        (if _returnvalue_2
          (`self.Toogle_widget` _hitactor)
          (set `self.Targeted_decal` (cast `/Game/RTS_Main/Blueprints/Decal/Decal_actor` _hitactor :!pure true))))))
  (:`Released`
    (`self.Unclick_widget`)))

(event `Main_hud_enable`
  ;[1 1 1] Begin Play
  (`UserWidget.AddToViewport` (`self.MainHud_Ref`) 0)
  (bind _asrts_game_mode (cast `/Game/RTS_Main/GameBP/rtsGameMode` (`GameplayStatics.GetGameMode`)))
  (`/Game/RTS_Main/GameBP/rtsGameMode.Start_game` _asrts_game_mode self))

(event `self.ReceiveBeginPlay`
  (bind _returnvalue (`KismetMathLibrary.MakeTransform` (0.0 0.0 0.0)))
  ;[1 1 1] Begin Play
  (`|ExecutionSequence`
    (:`then_0`
      (`self.ReferenceCasts`))
    (:`then_1`
      (bind _returnvalue_2 (`|SpawnActorFromClass` "/Game/RTS_Main/Blueprints/Construction/ConstructionManager_BP.ConstructionManager_BP_C" _returnvalue "AlwaysSpawn" "OverrideRootScale" null null))
      (set `self.ConstructionManagerRef` _returnvalue_2))
    (:`then_2`
      (bind _returnvalue_3 (`|SpawnActorFromClass` "/Game/RTS_Main/Blueprints/Buildings/GhostBuilding_BP.GhostBuilding_BP_C" _returnvalue "AlwaysSpawn" "OverrideRootScale" null self null))
      (set `self.GhostBuildingRef` _returnvalue_3))
    (:`then_3`
      (`WidgetBlueprintLibrary.SetInputMode_GameAndUIEx` self null "LockAlways" false)
      (`self.CreateHuds`)
      ;;[1 1 1] Disable color picker
      (if false
        (bind _returnvalue_4 (`|CreateWidget` "/Game/RTS_Main/HUDS/Color_picker.Color_picker_C" self self))
        (`UserWidget.AddToViewport` _returnvalue_4 0)
        (else
          (`self.Main_hud_enable`))))))

(event `InputAction|RotateBuildingRight`
  (params (Key :type "Key Structure"))
  (bind _ghostbuildingref (`self.GhostBuildingRef`))
  ;[1 1 1] . , Keys Building Rotate
  (:`Pressed`
    (if (and (`KismetSystemLibrary.IsValid` _ghostbuildingref) (`self.BuildModeActive`))
      (`self.K2_SetActorRotation` _ghostbuildingref (`KismetMathLibrary.MakeRotator` (.roll (`self.K2_GetActorRotation` _ghostbuildingref)) (.pitch (`self.K2_GetActorRotation` _ghostbuildingref)) (- (.yaw (`self.K2_GetActorRotation` _ghostbuildingref)) (`self.BuildingRotationRate`))) false))))

(event `InputAction|RotateBuildingLeft`
  (params (Key :type "Key Structure"))
  (bind _ghostbuildingref (`self.GhostBuildingRef`))
  ;[1 1 1] . , Keys Building Rotate
  (:`Pressed`
    (if (and (`KismetSystemLibrary.IsValid` _ghostbuildingref) (`self.BuildModeActive`))
      (`self.K2_SetActorRotation` _ghostbuildingref (`KismetMathLibrary.MakeRotator` (.roll (`self.K2_GetActorRotation` _ghostbuildingref)) (.pitch (`self.K2_GetActorRotation` _ghostbuildingref)) (+ (.yaw (`self.K2_GetActorRotation` _ghostbuildingref)) (`self.BuildingRotationRate`))) false))))

(event `InputAxis|MoveForward`
  (params (AxisValue :type "Float (single-precision)"))
  ;[0.2211 0.6 0.1184] Camera Movement
  ;;[1 1 1] X Movement
  (if (not (`self.DisableCamNav`))
    (`self.K2_SetActorTransform` (`self.CameraPawnRef`) (`self.MovementX` (`self.MovementSpeedCalculation`) (`self.FastMoveMultiplier`) AxisValue (`self.CameraPawnRef`)) true false)))

(event `InputAction|PanReset`
  (params (Key :type "Key Structure"))
  (bind _camerapawnref (`self.CameraPawnRef`))
  ;[0.2211 0.6 0.1184] Camera Movement
  ;;[1 1 1] Pan Reset
  (:`Pressed`
    (`self.K2_SetActorRotation` _camerapawnref (`KismetMathLibrary.MakeRotator` (.roll (`self.K2_GetActorRotation` _camerapawnref)) 0.0 (.yaw (`self.K2_GetActorRotation` _camerapawnref))) false)))

(event `InputAxis|MoveRight`
  (params (AxisValue :type "Float (single-precision)"))
  ;[0.2211 0.6 0.1184] Camera Movement
  ;;[1 1 1] Y Movement
  (if (not (`self.DisableCamNav`))
    (`self.K2_SetActorTransform` (`self.CameraPawnRef`) (`self.MovementY` AxisValue (`self.MovementSpeedCalculation`) (`self.FastMoveMultiplier`) (`self.CameraPawnRef`)) true false)))

(event `Key|V`
  (params (Key :type "Key Structure"))
  (bind (_mouselocation_x _mouselocation_y) (`KismetMathLibrary.BreakVector` (`/Game/RTS_Main/Libraries/FunctionLibrary.SetCursorWorldPosition` self 10000.0)))
  ;[1 1 1] V Key - Spawn NPC
  (:`Pressed`
    (`|SpawnActorFromClass` "/Game/RTS_Main/Blueprints/Buildings/Buildings_2_0/Tree.Tree_C" (`KismetMathLibrary.MakeTransform` (`KismetMathLibrary.MakeVector` _mouselocation_x _mouselocation_y 93.0)) "Undefined" "OverrideRootScale" null null)))

(event `Key|C`
  (params (Key :type "Key Structure"))
  (bind (_mouselocation_x _mouselocation_y) (`KismetMathLibrary.BreakVector` (`/Game/RTS_Main/Libraries/FunctionLibrary.SetCursorWorldPosition` self 10000.0)))
  (:`Pressed`
    (`|SpawnActorFromClass` "/Game/RTS_Main/Blueprints/Buildings/Buildings_2_0/Rock.Rock_C" (`KismetMathLibrary.MakeTransform` (`KismetMathLibrary.MakeVector` _mouselocation_x _mouselocation_y 93.0)) "Undefined" "OverrideRootScale" null null)))

(event `Change_energy`
  (params (NewParam :type Integer))
  ;[1 1 1] Add energy
  (set `self.Energy` (`KismetMathLibrary.Clamp` (+ (`self.Energy`) NewParam) 0 (`self.Max_energy`))))

(event `InputAxisKey|MouseX`
  (params (AxisValue :type "Float (single-precision)"))
  ;[0.2211 0.6 0.1184] Camera Movement
  ;;[1 1 1] Pan X
  (`/Engine/EditorBlueprintResources/StandardMacros.Gate` true :!label _label
    (:`Exit`
      (`self.K2_SetActorRotation` (`self.CameraPawnRef`) (`KismetMathLibrary.MakeRotator` (.roll (`self.K2_GetActorRotation` (`self.CameraPawnRef`))) (.pitch (`self.K2_GetActorRotation` (`self.CameraPawnRef`))) (+ (.yaw (`self.K2_GetActorRotation` (`self.CameraPawnRef`))) (* (`self.PanSensitivity`) AxisValue))) false))))

(event `Key|LeftShift`
  (params (Key :type "Key Structure"))
  ;[0.2211 0.6 0.1184] Camera Movement
  ;;[1 1 1] Move Multiplier
  (:`Pressed`
    (set `self.FastMoveMultiplier` 5.0))
  (:`Released`
    (set `self.FastMoveMultiplier` 1.0)))

(event `InputAction|Pan`
  (params (Key :type "Key Structure"))
  ;[0.2211 0.6 0.1184] Camera Movement
  ;;[1 1 1] Pan X
  (:`Pressed`
    (set `self.DisableCamNav` true)
    (goto _label :!via `Open`))
  (:`Released`
    (set `self.DisableCamNav` false)
    (goto _label :!via `Close`)))

(event `Key|Q`
  (params (Key :type "Key Structure"))
  (:`Pressed`
    (`/Engine/EditorBlueprintResources/StandardMacros.FlipFlop`
      (:`A`
        (set `self.Attack Mode` false)
        (set `self.BuildModeActive` false))
      (:`B`
        (set `self.Attack Mode` true)
        (set `self.BuildModeActive` true)
        (`SceneComponent.SetHiddenInGame` (`/Game/RTS_Main/Blueprints/CameraPawn.Grid` (`self.CameraPawnRef`)) true true)))))

(event `Key|P`
  (params (Key :type "Key Structure"))
  ;[1 1 1] P KEY Display UI timed
  (:`Pressed`
    (`|ExecutionSequence`
      (:`then_0`
        (bind _returnvalue (`|CreateWidget` "/Game/UltimateStatsComp/DemoData/Blueprints/WBP_DemoUSC_CustomCharacterInfoWindow.WBP_DemoUSC_CustomCharacterInfoWindow_C"))
        (`UserWidget.AddToViewport` _returnvalue 0))
      (:`then_1`
        (`KismetSystemLibrary.Delay` 5.0)
        (`WidgetLayoutLibrary.RemoveAllWidgets`)
        (bind _returnvalue_2 (`|CreateWidget` "/Game/RTS_Main/HUDS/MainUI.MainUI_C" self null (`self.GhostBuildingRef`) (`self.GameStateRef`)))
        (`UserWidget.AddToViewport` _returnvalue_2 0)))))

(event `InputAxisKey|MouseY`
  (params (AxisValue :type "Float (single-precision)"))
  ;[0.2211 0.6 0.1184] Camera Movement
  ;;[1 1 1] Pan Y
  (`/Engine/EditorBlueprintResources/StandardMacros.Gate` true :!label _label_2
    (:`Exit`
      (`self.K2_SetActorRotation` (`self.CameraPawnRef`) (`KismetMathLibrary.MakeRotator` (.roll (`self.K2_GetActorRotation` (`self.CameraPawnRef`))) (`KismetMathLibrary.FClamp` (+ (.pitch (`self.K2_GetActorRotation` (`self.CameraPawnRef`))) (* (`self.PanSensitivity`) AxisValue)) -5.0 25.0) (.yaw (`self.K2_GetActorRotation` (`self.CameraPawnRef`)))) false))))

(event `InputAction|Pan`
  (params (Key :type "Key Structure"))
  ;[0.2211 0.6 0.1184] Camera Movement
  ;;[1 1 1] Pan Y
  (:`Pressed`
    (set `self.DisableCamNav` true)
    (goto _label_2 :!via `Open`))
  (:`Released`
    (set `self.DisableCamNav` false)
    (goto _label_2 :!via `Close`)))

(event `InputAction|ZoomReset`
  (params (Key :type "Key Structure"))
  ;[0.2211 0.6 0.1184] Camera Movement
  ;;[1 1 1] Zoom Reset
  (:`Pressed`
    (set `SpringArmComponent.TargetArmLength` 1500.0 (`/Game/RTS_Main/Blueprints/CameraPawn.SpringArm` (`self.CameraPawnRef`)))))

(event `InputAction|Zoomin`
  (params (Key :type "Key Structure"))
  (bind _springarm (`/Game/RTS_Main/Blueprints/CameraPawn.SpringArm` (`self.CameraPawnRef`)))
  ;[0.2211 0.6 0.1184] Camera Movement
  ;;[1 1 1] Zoom In And out
  (:`Pressed`
    (set `SpringArmComponent.TargetArmLength` (`KismetMathLibrary.FClamp` (- (`SpringArmComponent.TargetArmLength` _springarm) (`self.ZoomSensitivity`)) 500.0 (`self.MaxArmDistance`)) _springarm)))

(event `InputAction|ZoomOut`
  (params (Key :type "Key Structure"))
  (bind _springarm (`/Game/RTS_Main/Blueprints/CameraPawn.SpringArm` (`self.CameraPawnRef`)))
  ;[0.2211 0.6 0.1184] Camera Movement
  ;;[1 1 1] Zoom In And out
  (:`Pressed`
    (set `SpringArmComponent.TargetArmLength` (`KismetMathLibrary.FClamp` (+ (`self.ZoomSensitivity`) (`SpringArmComponent.TargetArmLength` _springarm)) 500.0 (`self.MaxArmDistance`)) _springarm)))

(event `InputAxisKey|MouseX`
  (params (AxisValue :type "Float (single-precision)"))
  ;[0.2211 0.6 0.1184] Camera Movement
  ;;[1 1 1] Edge Movement
  (if (not (`self.DisableCamNav`))
    (bind (_deltaxspeed _deltayspeed) (`self.ScreenEdgeMovement` :!label _label_3))
    (`self.K2_AddActorLocalOffset` (`self.CameraPawnRef`) (`KismetMathLibrary.MakeVector` _deltaxspeed _deltayspeed) true false)))

(event `InputAxisKey|MouseY`
  (params (AxisValue :type "Float (single-precision)"))
  ;[0.2211 0.6 0.1184] Camera Movement
  ;;[1 1 1] Edge Movement
  (if (not (`self.DisableCamNav`))
    (goto _label_3 :!via `MouseY`)))

(event `self.ReceiveTick`
  (params (DeltaSeconds :type "Float (single-precision)"))
  ;[0.2211 0.6 0.1184] Camera Movement
  ;;[1 1 1] Cursor Position
  (if (`self.BuildModeActive`)
    (if (!= (`self.GhostBuildingRef`) null)
      (bind _newparam (`self.Get_location`))
      (`/Game/RTS_Main/Blueprints/CameraPawn.MoveGrid` (`self.CameraPawnRef`) _newparam)
      (`/Game/RTS_Main/Blueprints/Buildings/GhostBuilding_BP.SetCursorPosition` (`self.GhostBuildingRef`) _newparam))))

(event `InputAction|Deselect`
  (params (Key :type "Key Structure"))
  ;[0.2211 0.6 0.1184] Camera Movement
  (:`Pressed`
    (`self.Toogle_widget` (`self.Targeted_decal`) true)
    (if (`self.BuildModeActive`)
      (`/Game/RTS_Main/Blueprints/Buildings/GhostBuilding_BP.KillChost` (`self.GhostBuildingRef`))
      (set `self.BuildModeActive` false)
      (`SceneComponent.SetHiddenInGame` (`/Game/RTS_Main/Blueprints/CameraPawn.Grid` (`self.CameraPawnRef`)) true true)
      (set `self.Attack Mode` false))))

(fn `Click_widget`
  (`WidgetInteractionComponent.PressPointerKey` (`self.WidgetInteraction`) "LeftMouseButton")
  (return))

(fn `Get_location`
  (returns (NewParam :type "Vector Structure") (ReturnValue :type Boolean) (HitActor :type "Actor Object Reference"))
  (bind (_bblockinghit _binitialoverlap _time _distance _location _impactpoint _normal _impactnormal _physmat _hitactor) (`GameplayStatics.BreakHitResult` (`self.GetHitResultUnderCursorByChannel` "TraceTypeQuery2")))
  (return (`KismetMathLibrary.MakeVector` (`/Game/RTS_Main/Libraries/FunctionLibrary.GridSnap` (.x _location) 250) (`/Game/RTS_Main/Libraries/FunctionLibrary.GridSnap` (.y _location) 250) (`/Game/RTS_Main/Libraries/FunctionLibrary.GridSnap` (.z _location) 250)) (== (`GameplayStatics.GetObjectClass` _hitactor) "/Game/RTS_Main/Blueprints/Decal/Decal_actor.Decal_actor_C") _hitactor))

(fn `Have_energy?`
  (params (Decrement :type Integer))
  (returns (NewParam :type Boolean))
  (return (> (- (`self.Energy`) Decrement) 0)))

(fn `MovementSpeedCalculation`
  (returns (MoveSensitivity :type "Float (double-precision)"))
  (return (`KismetMathLibrary.FClamp` (/ (`SpringArmComponent.TargetArmLength` (`/Game/RTS_Main/Blueprints/CameraPawn.SpringArm` (`self.CameraPawnRef`))) 100.0) 5.0 20.0)))

(fn `SetCalendar`
  (params (Date :type "Array of Integer (by ref)"))
  (returns (Success :type Boolean))
  (return false))

(fn `SetClock`
  (params (Time :type "Array of Integer (by ref)"))
  (returns (Success :type Boolean))
  (return false))

(fn `SetSightDistance`
  (returns (SightDistance :type "Float (double-precision)"))
  (return (+ (`self.SightDistance`) (`SpringArmComponent.TargetArmLength` (`/Game/RTS_Main/Blueprints/CameraPawn.SpringArm` (`self.CameraPawnRef`))))))

(fn `Unclick_widget`
  (`WidgetInteractionComponent.ReleasePointerKey` (`self.WidgetInteraction`) "LeftMouseButton"))

(fn `UserConstructionScript`)