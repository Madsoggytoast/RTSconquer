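; ConstructionProxy_BP is a ghost-material stand-in for a building under construction, shown with a progress bar.
; The construction script applies the display mesh and sets up the entrance and collision box from it.
; Each tick accumulates clockwork time using a TimeUnit, with a game-speed update bound through the game state, and updates the Building_state widget.
; When work time reaches the construction time, it signals completion and destroys itself after a short delay.
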(event `self.ReceiveBeginPlay`
  (bind _output_get (set `self.GameStateRef` (cast `/Game/RTS_Main/GameBP/rtsGameState` (`GameplayStatics.GetGameState`) :!pure true)))
  (add `/Game/RTS_Main/GameBP/rtsGameState.UpdateGameSpeed` _output_get (`|CreateDelegate` :!event `AdjustTime`)))

(event `self.ReceiveTick`
  (params (DeltaSeconds :type "Float (single-precision)"))
  (set `self.Delta` DeltaSeconds)
  (if (not (`self.IsConstuctionCompleted`))
    (`self.DoWork`)
    (if (>= (`self.WorkTimeSpent`) (`self.ConstructionTime`))
      (set `self.IsConstuctionCompleted` true)
      (`self.ConstructionCompleted` self)
      (`KismetSystemLibrary.Delay` 0.2)
      (`self.K2_DestroyActor`))))

(event `AdjustTime`
  (params (TimeUnit :type "Float (double-precision)"))
  (set `self.TimeUnit` TimeUnit))

(fn `DoWork`
  (bind _output_get (set `self.ClockWork` (`/Game/RTS_Main/Libraries/FunctionLibrary.SetClockWork` (`self.Delta`) (`self.TimeUnit`) (`self.ClockWork`))))
  (bind _output_get_2 (set `self.WorkTimeSpent` (* _output_get 60.0)))
  ;[1 1 1] Progress Bar
  (bind _asbuilding_state (cast `/Game/RTS_Main/HUDS/Building_state` (`WidgetComponent.GetUserWidgetObject` (`self.Progress_bar`)))
    (:`then`
      (set `/Game/RTS_Main/HUDS/Building_state.Progress` (/ _output_get_2 (`self.ConstructionTime`)) _asbuilding_state))
    (:`CastFailed`
      _))
  (return))

(fn `SetConstructionTime`
  (params (WorkHours :type "Float (double-precision)"))
  (set `self.ConstructionTime` (* WorkHours 60.0))
  (return))

(fn `UserConstructionScript`
  (bind _staticmesh (`self.StaticMesh`))
  (`StaticMeshComponent.SetStaticMesh` _staticmesh (`self.DisplayMesh`))
  (`PrimitiveComponent.SetMaterial` _staticmesh 0 "/Game/RTS_Main/Materials/Ghost_M_Inst.Ghost_M_Inst")
  (`/Game/RTS_Main/Libraries/FunctionLibrary.SetBuildingEntrance` (`self.Entrance`) (`self.StaticMesh`))
  (`/Game/RTS_Main/Libraries/FunctionLibrary.SetBuildingCollisionBox` (`self.Collision`) (`self.StaticMesh`)))