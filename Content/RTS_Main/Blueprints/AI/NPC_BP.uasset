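; NPC Blueprint for the RTS that randomizes its appearance in the construction script, with no active event logic.
; RandomNPCFeatures creates a dynamic body material and tints it male or female color from a random sex roll.
; GetRandomName picks a random enum entry as a name, but its hardcoded branch ignores Sex and always takes the male list.
; The MyProfile writes are unconnected, so name and sex are never stored.
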(fn `GetRandomName`
  (params (Sex :type "/Game/RTS_Main/Enums/NPCSexType_ENUM Enum" :default "NewEnumerator0"))
  (returns (Name :type String))
  (if true
    (return (`|GetEnumeratorNameAsString` (enumliteral `/Game/RTS_Main/Enums/NPCMaleName_ENUM` (cast `/Game/RTS_Main/Enums/NPCMaleName_ENUM` (`KismetMathLibrary.Conv_IntToByte` (`KismetMathLibrary.RandomIntegerInRange` 1 (- (enumcount `/Game/RTS_Main/Enums/NPCMaleName_ENUM`) 1)))))))
    (else
      (return (`|GetEnumeratorNameAsString` (enumliteral `/Game/RTS_Main/Enums/NCPNameFemale_ENUM` (cast `/Game/RTS_Main/Enums/NCPNameFemale_ENUM` (`KismetMathLibrary.Conv_IntToByte` (`KismetMathLibrary.RandomIntegerInRange` 1 (- (enumcount `/Game/RTS_Main/Enums/NCPNameFemale_ENUM`) 1))))))))))

(fn `RandomNPCFeatures`
  (locals (MaterialInstance :type "MaterialInstanceDynamic Object Reference") (FemaleColor :type "LinearColor Structure" :default (struct :`R` 0.451 :`G` 0.028 :`B` 0.266)) (MaleColor :type "LinearColor Structure" :default (struct :`R` 0.026007 :`G` 0.075525 :`B` 0.445833)))
  (bind _materialinstance (`local.MaterialInstance`))
  (bind _returnvalue (`PrimitiveComponent.CreateDynamicMaterialInstance` (`self.Mesh`) 0 "/Game/Mannequin/Character/Materials/M_UE4Man_Body_Inst.M_UE4Man_Body_Inst"))
  (set `local.MaterialInstance` _returnvalue)
  (if (`|EnumEquality` (enumliteral `/Game/RTS_Main/Enums/NPCSexType_ENUM` (cast `/Game/RTS_Main/Enums/NPCSexType_ENUM` (`KismetMathLibrary.Conv_IntToByte` (`KismetMathLibrary.RandomIntegerInRange` 0 1)))) "NewEnumerator0")
    (`MaterialInstanceDynamic.SetVectorParameterValue` _materialinstance "BodyColor" (`local.MaleColor`))
    (bind _name (`self.GetRandomName` "NewEnumerator0"))
    (else
      (`MaterialInstanceDynamic.SetVectorParameterValue` _materialinstance "BodyColor" (`local.FemaleColor`))
      (bind _name_2 (`self.GetRandomName` "NewEnumerator1")))))

(fn `UserConstructionScript`
  (`self.RandomNPCFeatures`))