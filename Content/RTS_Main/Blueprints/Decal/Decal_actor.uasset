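; Decal actor for the RTS that shows a decal tinted in a player color and carries an Actions_possible widget.
; On BeginPlay it creates a dynamic material instance on the decal and sets its Color parameter from the RGB of PlayerColor.
; It then casts the widget component's user widget to Actions_possible and sets itself as that widget's Owner.
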(event `self.ReceiveBeginPlay`
  (bind (_r _g _b) (break `LinearColor` (`.SpecifiedColor` (break `SlateColor` (`self.Player_color`)))))
  (bind _returnvalue (`DecalComponent.CreateDynamicMaterialInstance` (`self.Decal`)))
  (`MaterialInstanceDynamic.SetVectorParameterValue` _returnvalue "Color" (`KismetMathLibrary.MakeColor` _r _g _b))
  (bind _asactions_possible (cast `/Game/RTS_Main/HUDS/Actions_possible` (`WidgetComponent.GetUserWidgetObject` (`self.Widget`))))
  (set `/Game/RTS_Main/HUDS/Actions_possible.Owner` self _asactions_possible))

(fn `UserConstructionScript`)