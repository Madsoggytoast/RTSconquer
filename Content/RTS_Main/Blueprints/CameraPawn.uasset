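; RTS camera pawn that carries a Grid component which can be placed at a given world position.
; MoveGrid unhides the grid and moves it to the supplied location, raised slightly in Z.
; A Box component clears the Blocking flag when an overlap ends.
; The logic that would set Blocking for BlockingVolume actors is disconnected, so overlap begin does nothing.
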(event `MoveGrid`
  (params (NewParam :type "Vector Structure"))
  (if (`SceneComponent.bHiddenInGame` (`self.Grid`))
    (`SceneComponent.SetHiddenInGame` (`self.Grid`) false true))
  (`SceneComponent.K2_SetWorldLocation` (`self.Grid`) (`KismetMathLibrary.MakeVector` (.x NewParam) (.y NewParam) (+ (.z NewParam) 10.0)) false false))

(event `self.Box.OnComponentBeginOverlap`
  (params (OverlappedComponent :type "PrimitiveComponent Object Reference") (OtherActor :type "Actor Object Reference") (OtherComp :type "PrimitiveComponent Object Reference") (OtherBodyIndex :type Integer) (bFromSweep :type Boolean) (SweepResult :type "HitResult Structure (by ref)")))

(event `self.Box.OnComponentEndOverlap`
  (params (OverlappedComponent :type "PrimitiveComponent Object Reference") (OtherActor :type "Actor Object Reference") (OtherComp :type "PrimitiveComponent Object Reference") (OtherBodyIndex :type Integer))
  (set `self.Blocking` false))

(fn `UserConstructionScript`)