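; Blueprint function library for the UltimateStatsComp stats system, providing display and math helpers.
; Select-based lookups map attribute, stat, buff and effect enums to display text, and buff and effect enums also to icons.
; Duration conversion turns seconds into a minutes:seconds text, using a helper that zero-pads single-digit seconds.
; Two more helpers sum integer and float arrays.
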(fn `AddUpAllArrayFloats`
  (params (Array :type "Array of Float (double-precision)"))
  (returns (Result :type "Float (double-precision)"))
  (locals (ResultLOCAL :type "Float (double-precision)"))
  (for _array_element Array
    (set `local.ResultLOCAL` (+ _array_element (`local.ResultLOCAL`))))
  (return (`local.ResultLOCAL`)))

(fn `AddUpAllArrayIntegers`
  (params (Array :type "Array of Integer"))
  (returns (Result :type Integer))
  (locals (ResultLOCAL :type Integer))
  (for _array_element Array
    (set `local.ResultLOCAL` (+ _array_element (`local.ResultLOCAL`))))
  (return (`local.ResultLOCAL`)))

(fn `AttributeTypeToText`
  (params (AttributeType :type "/Game/UltimateStatsComp/Enumerations/E_USC_AttributeType Enum" :default "NewEnumerator4"))
  (returns (Text :type Text))
  (return (select `/Game/UltimateStatsComp/Enumerations/E_USC_AttributeType` AttributeType :`NewEnumerator4` "Non Available" :`NewEnumerator0` "Strength" :`NewEnumerator1` "Dexterity" :`NewEnumerator2` "Endurance" :`NewEnumerator3` "Wisdom" :!type "Text")))

(fn `BuffTypeToImage`
  (params (BuffType :type "/Game/UltimateStatsComp/Enumerations/E_USC_BuffType Enum" :default "NewEnumerator0"))
  (returns (Texture :type "Texture2D Object Reference"))
  (return (select `/Game/UltimateStatsComp/Enumerations/E_USC_BuffType` BuffType :`NewEnumerator0` "/Game/UltimateStatsComp/DemoData/Icons/Buffs/I_Buff_Toughness.I_Buff_Toughness" :`NewEnumerator1` "/Game/UltimateStatsComp/DemoData/Icons/Buffs/I_Buff_Haste.I_Buff_Haste" :`NewEnumerator2` "/Game/UltimateStatsComp/DemoData/Icons/Buffs/I_Buff_LuckyDice.I_Buff_LuckyDice" :`NewEnumerator5` "/Game/UltimateStatsComp/DemoData/Icons/Buffs/I_Buff_Warcry.I_Buff_Warcry" :!type "Texture2D Object Reference")))

(fn `BuffTypeToText`
  (params (BuffType :type "/Game/UltimateStatsComp/Enumerations/E_USC_BuffType Enum" :default "NewEnumerator0"))
  (returns (Text :type Text))
  (return (select `/Game/UltimateStatsComp/Enumerations/E_USC_BuffType` BuffType :`NewEnumerator0` "Toughness" :`NewEnumerator1` "Haste" :`NewEnumerator2` "Lucky Dice" :`NewEnumerator5` "Warcry" :!type "Text")))

(fn `DurationTimeConversion`
  (params (Duration :type "Float (double-precision)"))
  (returns (BuffDurationInText :type Text))
  (bind (_remainder _returnvalue) (`KismetMathLibrary.FMod` Duration 60.0))
  (return (`|FormatText` "{minutes}:{seconds}" _returnvalue (`self.SingleDigitToDoubleNumber` (`KismetMathLibrary.FTrunc` _remainder)))))

(fn `EffectTypeToImage`
  (params (EffectType :type "/Game/UltimateStatsComp/Enumerations/E_USC_EffectType Enum" :default "NewEnumerator0"))
  (returns (Texture :type "Texture2D Object Reference"))
  (return (select `/Game/UltimateStatsComp/Enumerations/E_USC_EffectType` EffectType :`NewEnumerator0` "/Game/UltimateStatsComp/DemoData/Icons/Effects/I_Effect_HealthRegeneration.I_Effect_HealthRegeneration" :`NewEnumerator1` "/Game/UltimateStatsComp/DemoData/Icons/Effects/I_Effect_Burning.I_Effect_Burning" :`NewEnumerator2` "/Game/UltimateStatsComp/DemoData/Icons/Effects/I_Effect_Poisoning.I_Effect_Poisoning" :`NewEnumerator3` "/Game/UltimateStatsComp/DemoData/Icons/Effects/I_Effect_ManaRegeneration.I_Effect_ManaRegeneration" :!type "Texture2D Object Reference")))

(fn `EffectTypeToText`
  (params (EffectType :type "/Game/UltimateStatsComp/Enumerations/E_USC_EffectType Enum" :default "NewEnumerator0"))
  (returns (Text :type Text))
  (return (select `/Game/UltimateStatsComp/Enumerations/E_USC_EffectType` EffectType :`NewEnumerator0` "Health Regeneration" :`NewEnumerator1` "Burning" :`NewEnumerator2` "Poisoning" :`NewEnumerator3` "Mana Regeneration" :!type "Text")))

(fn `SingleDigitToDoubleNumber`
  (params (Number :type Integer))
  (returns (DoubleDigitNumber :type Text))
  (bind _returnvalue (`KismetStringLibrary.Conv_IntToString` Number))
  (return (select `bool` (> (`KismetStringLibrary.Len` _returnvalue) 1) :`false` (`KismetTextLibrary.Conv_StringToText` (`KismetStringLibrary.Concat_StrStr` "0" _returnvalue)) :`true` (`KismetTextLibrary.Conv_StringToText` _returnvalue))))

(fn `StatTypeToText`
  (params (StatType :type "/Game/UltimateStatsComp/Enumerations/E_USC_StatType Enum" :default "NewEnumerator0"))
  (returns (Text :type Text))
  (return (select `/Game/UltimateStatsComp/Enumerations/E_USC_StatType` StatType :`NewEnumerator0` "Non Available" :`NewEnumerator1` "Health" :`NewEnumerator2` "Mana" :`NewEnumerator3` "Power" :`NewEnumerator4` "Movement Speed" :`NewEnumerator5` "Critical Rate" :`NewEnumerator6` "Critical Power" :`NewEnumerator7` "Defence" :!type "Text")))