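; Demo player controller for the Ultimate Stats Component, wiring the controlled character to its stats UI and input.
; On authority it polls for the pawn, then client and server events build the HUD and stats widgets, load saved stats and refresh bars.
; Key-set axis scales drive movement on Tick, while mouse axes turn the view.
; Keys toggle the info window and pause, navigate attribute, stat and buff slots, and spend points.
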(event `self.ReceiveBeginPlay`
  ;[0.3 0.3 0.3] Initialization
  (`/Engine/EditorBlueprintResources/ActorMacros.Switch Has Authority`
    (:`Authority`
      ;;[1 1 1 1 12] Create Reference to Player Character (if it is mutliplayer game reference will be created only on server side)
      (bind _asbp_demo_usc_character (cast `/Game/UltimateStatsComp/DemoData/Blueprints/BP_DemoUSC_Character` (`self.K2_GetPawn`) :!label _label)
        (:`then`
          (set `/Game/UltimateStatsComp/DemoData/Blueprints/BP_DemoUSC_Character.ControllerReference` self _asbp_demo_usc_character)
          (set `self.ControlledCharacterReference` _asbp_demo_usc_character)
          (`self.CreateWidgets_CLIENT`) ; Creates necessary widgets (Multiplayer: creates widgets only on client)
        )
        (:`CastFailed`
          (`KismetSystemLibrary.Delay` 0.2)
          (goto _label))))))

(event `CreateWidgets_CLIENT`
  (bind _ac_usc_stats (`/Game/UltimateStatsComp/DemoData/Blueprints/BP_DemoUSC_Character.AC_USC_Stats` (`self.ControlledCharacterReference`)))
  ;[0.3 0.3 0.3] Initialization
  (`WidgetBlueprintLibrary.SetInputMode_GameOnly` self)
  ;;[1 1 1 1 12] Creates basic HUD
  (bind _returnvalue (`|CreateWidget` "/Game/UltimateStatsComp/DemoData/Blueprints/WBP_DemoUSC_CustomCharacterInfoWindow.WBP_DemoUSC_CustomCharacterInfoWindow_C"))
  (bind _output_get (set `self.HUDReference` _returnvalue))
  (`UserWidget.AddToViewport` _output_get 0)
  (`Widget.SetVisibility` (`/Game/UltimateStatsComp/DemoData/Blueprints/WBP_DemoUSC_CustomCharacterInfoWindow.Box_StatsWindow` (`self.HUDReference`)) "Collapsed") ; Characters stats info window shouldn't be shown at start
  (`self.ControlledCharacterReference`
    (:`then`
      _)
    (:`else`
      ;;[1 1 1 1 12] Wait for pawn if it still doesn't exist. (creates reference to controlled character on client side if it is multiplayer game).
      (bind _asbp_demo_usc_character (cast `/Game/UltimateStatsComp/DemoData/Blueprints/BP_DemoUSC_Character` (`self.K2_GetPawn`) :!label _label_2)
        (:`then`
          (set `/Game/UltimateStatsComp/DemoData/Blueprints/BP_DemoUSC_Character.ControllerReference` self _asbp_demo_usc_character)
          (set `self.ControlledCharacterReference` _asbp_demo_usc_character))
        (:`CastFailed`
          (`KismetSystemLibrary.Delay` 0.2)
          (goto _label_2)))))
  ;;[1 1 1 1 12] Creates necessary widgets from StatsComponent (Multiplayer: it is executed only on client side)
  (`/Game/UltimateStatsComp/Blueprints/AC_USC_Stats.CreateAttributesWindow` _ac_usc_stats)
  (`/Game/UltimateStatsComp/Blueprints/AC_USC_Stats.CreateStatsWindow` _ac_usc_stats)
  (`/Game/UltimateStatsComp/Blueprints/AC_USC_Stats.CreateBuffsAndEffectsBar` _ac_usc_stats)
  (`/Game/UltimateStatsComp/Blueprints/AC_USC_Stats.InitialWindowsUpdate` _ac_usc_stats)
  (`self.UpdateAttributesAndStats_SERVER`) ; Read character stats values and updates corresponding widgets\n(Multiplayer: data is read from server and send to client)
)

(event `UpdateAttributesAndStats_SERVER`
  (bind _controlledcharacterreference (`self.ControlledCharacterReference`))
  (bind _ac_usc_stats (`/Game/UltimateStatsComp/DemoData/Blueprints/BP_DemoUSC_Character.AC_USC_Stats` (`self.ControlledCharacterReference`)))
  (bind _ac_usc_stats_2 (`/Game/UltimateStatsComp/DemoData/Blueprints/BP_DemoUSC_Character.AC_USC_Stats` (`self.ControlledCharacterReference`)))
  ;[0.3 0.3 0.3] Initialization
  (`/Game/UltimateStatsComp/Blueprints/AC_USC_Stats.ScaleAttributesAndStatsWithLevel` (`/Game/UltimateStatsComp/DemoData/Blueprints/BP_DemoUSC_Character.AC_USC_Stats` (`self.ControlledCharacterReference`))) ; Execute "Scaling" function before loading stats data will assign default stats to actor.\nIf there is no proper data to load, character will stick to default stats.\n However if save data exists default stats will be simply overwritten with the ones from save data.
  (`/Game/UltimateStatsComp/Blueprints/AC_USC_Stats.LoadStatsData` (`/Game/UltimateStatsComp/DemoData/Blueprints/BP_DemoUSC_Character.AC_USC_Stats` (`self.ControlledCharacterReference`)) "DemoCharacter_Stats" true)
  (`/Game/UltimateStatsComp/Blueprints/AC_USC_Stats.PerformFullAttributesAndStatsRecalculation` (`/Game/UltimateStatsComp/DemoData/Blueprints/BP_DemoUSC_Character.AC_USC_Stats` (`self.ControlledCharacterReference`))) ; Recalculate all stats after loading
  (`/Game/UltimateStatsComp/Blueprints/AC_USC_Stats.InitialWindowsUpdate` (`/Game/UltimateStatsComp/DemoData/Blueprints/BP_DemoUSC_Character.AC_USC_Stats` (`self.ControlledCharacterReference`)))
  ;;[1 1 1 1 12] Additional widgets updates (this updates custom widget such as Health/Mana Bars and level/XP bar located at the bottom of the screen).
  (`/Game/UltimateStatsComp/DemoData/Blueprints/BP_DemoUSC_Character.UpdateHealthBar_CLIENT` _controlledcharacterreference (`BlueprintMapLibrary.Map_Find` (`/Game/UltimateStatsComp/Blueprints/AC_USC_Stats.CurrentStats` _ac_usc_stats) "NewEnumerator1") (`.FinalValue_9_72CA6EAC410161A8DBACDEA210F24628` (break `/Game/UltimateStatsComp/Structures/S_USC_BaseStat` (`BlueprintMapLibrary.Map_Find` (`/Game/UltimateStatsComp/Blueprints/AC_USC_Stats.BaseStats` _ac_usc_stats) "NewEnumerator1"))))
  (`/Game/UltimateStatsComp/DemoData/Blueprints/BP_DemoUSC_Character.UpdateManaBar_CLIENT` _controlledcharacterreference (`BlueprintMapLibrary.Map_Find` (`/Game/UltimateStatsComp/Blueprints/AC_USC_Stats.CurrentStats` _ac_usc_stats_2) "NewEnumerator2") (`.FinalValue_9_72CA6EAC410161A8DBACDEA210F24628` (break `/Game/UltimateStatsComp/Structures/S_USC_BaseStat` (`BlueprintMapLibrary.Map_Find` (`/Game/UltimateStatsComp/Blueprints/AC_USC_Stats.BaseStats` _ac_usc_stats_2) "NewEnumerator2"))))
  (`/Game/UltimateStatsComp/DemoData/Blueprints/BP_DemoUSC_Character.UpdateLevel_CLIENT` _controlledcharacterreference (`/Game/UltimateStatsComp/Blueprints/AC_USC_Stats.CurrentLevel` (`/Game/UltimateStatsComp/DemoData/Blueprints/BP_DemoUSC_Character.AC_USC_Stats` (`self.ControlledCharacterReference`)))))

(event `self.ReceiveTick`
  (params (DeltaSeconds :type "Float (single-precision)"))
  (bind (_returnvalue_roll _returnvalue_pitch _returnvalue_yaw) (`KismetMathLibrary.BreakRotator` (`self.GetControlRotation`)))
  ;[1 1 1] Movement is bound to tick event, so it won't require special input commands set from user.
  (bind _controlledcharacterreference (`self.ControlledCharacterReference`)
    (:`then`
      (`Pawn.AddMovementInput` _controlledcharacterreference (`KismetMathLibrary.GetForwardVector` (`KismetMathLibrary.MakeRotator` 0.0 0.0 _returnvalue_yaw)) (`self.ForwardMovementScale`) false)
      (`Pawn.AddMovementInput` _controlledcharacterreference (`KismetMathLibrary.GetRightVector` (`KismetMathLibrary.MakeRotator` 0.0 0.0 _returnvalue_yaw)) (`self.RightMovementScale`) false))
    (:`else`)))

(event `InputAxisKey|MouseX`
  (params (AxisValue :type "Float (single-precision)"))
  (`self.AddYawInput` AxisValue))

(event `InputAxisKey|MouseY`
  (params (AxisValue :type "Float (single-precision)"))
  (`self.AddPitchInput` (* AxisValue -1.0)))

(event `Key|W`
  (params (Key :type "Key Structure"))
  (:`Pressed`
    (set `self.ForwardMovementScale` 1.0))
  (:`Released`
    (set `self.ForwardMovementScale` 0.0)))

(event `Key|S`
  (params (Key :type "Key Structure"))
  (:`Pressed`
    (set `self.ForwardMovementScale` -1.0))
  (:`Released`
    (set `self.ForwardMovementScale` 0.0)))

(event `Key|D`
  (params (Key :type "Key Structure"))
  (:`Pressed`
    (set `self.RightMovementScale` 1.0))
  (:`Released`
    (set `self.RightMovementScale` 0.0)))

(event `Key|A`
  (params (Key :type "Key Structure"))
  (:`Pressed`
    (set `self.RightMovementScale` -1.0))
  (:`Released`
    (set `self.RightMovementScale` 0.0)))

(event `Key|Up`
  (params (Key :type "Key Structure"))
  (:`Pressed`
    (bind _controlledcharacterreference (`self.ControlledCharacterReference`)
      (:`then`
        (bind _ac_usc_stats (`/Game/UltimateStatsComp/DemoData/Blueprints/BP_DemoUSC_Character.AC_USC_Stats` _controlledcharacterreference))
        (switch `/Game/UltimateStatsComp/Enumerations/E_USC_SelectedWidget` (`/Game/UltimateStatsComp/Blueprints/AC_USC_Stats.CurrentlySelectedWidget` _ac_usc_stats)
          (:`NewEnumerator0`
            (`/Game/UltimateStatsComp/Blueprints/AC_USC_Stats.SelectPreviousAttributeSlot` _ac_usc_stats))
          (:`NewEnumerator1`
            (bind _successful_ (`/Game/UltimateStatsComp/Blueprints/AC_USC_Stats.SelectPreviousStatSlot` _ac_usc_stats))
            (if (not _successful_)
              (`/Game/UltimateStatsComp/Blueprints/AC_USC_Stats.SwitchToAttributesWindow` (`/Game/UltimateStatsComp/DemoData/Blueprints/BP_DemoUSC_Character.AC_USC_Stats` (`self.ControlledCharacterReference`)) 3)))))
      (:`else`))))

(event `Key|Down`
  (params (Key :type "Key Structure"))
  (:`Pressed`
    (bind _controlledcharacterreference (`self.ControlledCharacterReference`)
      (:`then`
        (bind _ac_usc_stats (`/Game/UltimateStatsComp/DemoData/Blueprints/BP_DemoUSC_Character.AC_USC_Stats` _controlledcharacterreference))
        (switch `/Game/UltimateStatsComp/Enumerations/E_USC_SelectedWidget` (`/Game/UltimateStatsComp/Blueprints/AC_USC_Stats.CurrentlySelectedWidget` _ac_usc_stats)
          (:`NewEnumerator0`
            (bind _successful_ (`/Game/UltimateStatsComp/Blueprints/AC_USC_Stats.SelectNextAttributeSlot` _ac_usc_stats))
            (if (not _successful_)
              (`/Game/UltimateStatsComp/Blueprints/AC_USC_Stats.SwitchToStatsWindow` (`/Game/UltimateStatsComp/DemoData/Blueprints/BP_DemoUSC_Character.AC_USC_Stats` (`self.ControlledCharacterReference`)) 0)))
          (:`NewEnumerator1`
            (`/Game/UltimateStatsComp/Blueprints/AC_USC_Stats.SelectNextStatSlot` _ac_usc_stats))))
      (:`else`))))

(event `Key|Left`
  (params (Key :type "Key Structure"))
  (:`Pressed`
    (bind _controlledcharacterreference (`self.ControlledCharacterReference`)
      (:`then`
        (bind _ac_usc_stats (`/Game/UltimateStatsComp/DemoData/Blueprints/BP_DemoUSC_Character.AC_USC_Stats` _controlledcharacterreference))
        (switch `/Game/UltimateStatsComp/Enumerations/E_USC_SelectedWidget` (`/Game/UltimateStatsComp/Blueprints/AC_USC_Stats.CurrentlySelectedWidget` _ac_usc_stats)
          (:`NewEnumerator2`
            (bind _successful_ (`/Game/UltimateStatsComp/Blueprints/AC_USC_Stats.SelectPreviousBuffOrEffectSlot` _ac_usc_stats))
            (if (not _successful_)
              (`/Game/UltimateStatsComp/Blueprints/AC_USC_Stats.SwitchToAttributesWindow` (`/Game/UltimateStatsComp/DemoData/Blueprints/BP_DemoUSC_Character.AC_USC_Stats` (`self.ControlledCharacterReference`)) 0)))))
      (:`else`))))

(event `Key|Right`
  (params (Key :type "Key Structure"))
  (:`Pressed`
    (bind _controlledcharacterreference (`self.ControlledCharacterReference`)
      (:`then`
        (bind _ac_usc_stats (`/Game/UltimateStatsComp/DemoData/Blueprints/BP_DemoUSC_Character.AC_USC_Stats` _controlledcharacterreference))
        (switch `/Game/UltimateStatsComp/Enumerations/E_USC_SelectedWidget` (`/Game/UltimateStatsComp/Blueprints/AC_USC_Stats.CurrentlySelectedWidget` _ac_usc_stats)
          (:`NewEnumerator0`
            (`/Game/UltimateStatsComp/Blueprints/AC_USC_Stats.SwitchToBuffsAndEffectsBar` (`/Game/UltimateStatsComp/DemoData/Blueprints/BP_DemoUSC_Character.AC_USC_Stats` (`self.ControlledCharacterReference`)) 0 :!label _label) ; Pressing right anytime in stats or attributes windows\nwill switch to buffs/effects bar.
          )
          (:`NewEnumerator1`
            (goto _label))
          (:`NewEnumerator2`
            (`/Game/UltimateStatsComp/Blueprints/AC_USC_Stats.SelectNextBuffOrEffectSlot` _ac_usc_stats))))
      (:`else`))))

(event `Key|SpaceBar`
  (params (Key :type "Key Structure"))
  ;[1 1 1] Spent attribute point with gamepad
  (:`Pressed`
    (bind _controlledcharacterreference (`self.ControlledCharacterReference`)
      (:`then`
        (`/Game/UltimateStatsComp/Blueprints/AC_USC_Stats.IncreaseAttributeByGamepad` (`/Game/UltimateStatsComp/DemoData/Blueprints/BP_DemoUSC_Character.AC_USC_Stats` _controlledcharacterreference)))
      (:`else`))))

(event `Key|C`
  (params (Key :type "Key Structure"))
  ;[1 1 1] Toggle Character Info Window
  (:`Pressed`
    (bind _hudreference (`self.HUDReference`)
      (:`then`
        (switch `ESlateVisibility` (`Widget.GetVisibility` (`/Game/UltimateStatsComp/DemoData/Blueprints/WBP_DemoUSC_CustomCharacterInfoWindow.Box_StatsWindow` _hudreference))
          (:`Visible`
            (`Widget.SetVisibility` (`/Game/UltimateStatsComp/DemoData/Blueprints/WBP_DemoUSC_CustomCharacterInfoWindow.Box_StatsWindow` (`self.HUDReference`)) "Collapsed" :!label _label_2)
            (`WidgetBlueprintLibrary.SetInputMode_GameOnly` self)
            (if (`/Game/UltimateStatsComp/Blueprints/AC_USC_Stats.UseGamepad?` (`/Game/UltimateStatsComp/DemoData/Blueprints/BP_DemoUSC_Character.AC_USC_Stats` (`self.ControlledCharacterReference`)))
              (`/Game/UltimateStatsComp/Blueprints/AC_USC_Stats.DeactivateGamepadSelection` (`/Game/UltimateStatsComp/DemoData/Blueprints/BP_DemoUSC_Character.AC_USC_Stats` (`self.ControlledCharacterReference`)))
              (else
                (set `self.bShowMouseCursor` false))))
          (:`Collapsed`
            (`Widget.SetVisibility` (`/Game/UltimateStatsComp/DemoData/Blueprints/WBP_DemoUSC_CustomCharacterInfoWindow.Box_StatsWindow` (`self.HUDReference`)) "SelfHitTestInvisible" :!label _label_3)
            (`WidgetBlueprintLibrary.SetInputMode_GameAndUIEx` self)
            (if (`/Game/UltimateStatsComp/Blueprints/AC_USC_Stats.UseGamepad?` (`/Game/UltimateStatsComp/DemoData/Blueprints/BP_DemoUSC_Character.AC_USC_Stats` (`self.ControlledCharacterReference`)))
              (`/Game/UltimateStatsComp/Blueprints/AC_USC_Stats.ActivateGamepadSelection` (`/Game/UltimateStatsComp/DemoData/Blueprints/BP_DemoUSC_Character.AC_USC_Stats` (`self.ControlledCharacterReference`)))
              (else
                (set `self.bShowMouseCursor` true))))
          (:`Hidden`
            (goto _label_3))
          (:`HitTestInvisible`
            (goto _label_2))
          (:`SelfHitTestInvisible`
            (goto _label_2))))
      (:`else`))))

(event `Key|P` :paused true
  (params (Key :type "Key Structure"))
  ;[1 1 1] Pause
  (:`Pressed`
    (if (`GameplayStatics.IsGamePaused`)
      (`GameplayStatics.SetGamePaused` false)
      (else
        (`GameplayStatics.SetGamePaused` true)))))

(fn `UserConstructionScript`)