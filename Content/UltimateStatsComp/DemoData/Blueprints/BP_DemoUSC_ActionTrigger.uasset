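; BP_DemoUSC_ActionTrigger is a demo actor for UltimateStatsComp that shows a floating text label facing the player.
; The construction script applies the CustomText and TextSize variables to the TextRender component.
; Each Tick casts the player character to BP_DemoUSC_Character and turns the text in yaw only toward its FollowCamera.
; No trigger or overlap logic is implemented in these graphs.
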(event `self.ReceiveTick`
  (params (DeltaSeconds :type "Float (single-precision)"))
  (bind _asbp_demo_usc_character (cast `/Game/UltimateStatsComp/DemoData/Blueprints/BP_DemoUSC_Character` (`GameplayStatics.GetPlayerCharacter` 0)))
  (bind (_returnvalue_roll _returnvalue_pitch _returnvalue_yaw) (`KismetMathLibrary.BreakRotator` (`KismetMathLibrary.FindLookAtRotation` (`SceneComponent.K2_GetComponentLocation` (`self.TextRender`)) (`SceneComponent.K2_GetComponentLocation` (`/Game/UltimateStatsComp/DemoData/Blueprints/BP_DemoUSC_Character.FollowCamera` _asbp_demo_usc_character)))))
  (`SceneComponent.K2_SetWorldRotation` (`self.TextRender`) (`KismetMathLibrary.MakeRotator` 0.0 0.0 _returnvalue_yaw) false false))

(fn `UserConstructionScript`
  (bind _textrender (`self.TextRender`))
  (`TextRenderComponent.K2_SetText` _textrender (`self.CustomText`))
  (`TextRenderComponent.SetWorldSize` _textrender (`self.TextSize`)))