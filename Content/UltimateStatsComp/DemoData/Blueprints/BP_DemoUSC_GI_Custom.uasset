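; Demo game instance for the Ultimate Stats Component that carries actor stats in memory and handles menus, sessions and graphics presets.
; Stats components save their data struct into a map keyed by save name and read it back on load.
; Menu events show widgets, mostly cached, while session events host a listen-server Lobby, join or destroy sessions.
; Low, medium and high presets apply scalability through console commands.
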(event `Low_Settings`
  ;[1 1 1] Game graphics
  (`KismetSystemLibrary.ExecuteConsoleCommand` "r.screenpercentage 50")
  (`KismetSystemLibrary.ExecuteConsoleCommand` "r.ViewDistanceScale 0.4")
  (`KismetSystemLibrary.ExecuteConsoleCommand` "r.PostProcessAAQuality 2")
  (`KismetSystemLibrary.ExecuteConsoleCommand` "sg.PostProcessQuality 0")
  (`KismetSystemLibrary.ExecuteConsoleCommand` "sg.ShadowQuality 0")
  (`KismetSystemLibrary.ExecuteConsoleCommand` "sg.TextureQuality 0")
  (`KismetSystemLibrary.ExecuteConsoleCommand` "FoliageQuality 0")
  (`KismetSystemLibrary.ExecuteConsoleCommand` "sg.EffectsQuality 0"))

(event `Medium_Settings`
  ;[1 1 1] Game graphics
  (`KismetSystemLibrary.ExecuteConsoleCommand` "r.ScreenPercentage 75%")
  (`KismetSystemLibrary.ExecuteConsoleCommand` "r.ViewDistanceScale 0.7")
  (`KismetSystemLibrary.ExecuteConsoleCommand` "r.PostProcessAAQuality 4")
  (`KismetSystemLibrary.ExecuteConsoleCommand` "sg.PostProcessQuality 1")
  (`KismetSystemLibrary.ExecuteConsoleCommand` "sg.ShadowQuality 1")
  (`KismetSystemLibrary.ExecuteConsoleCommand` "sg.TextureQuality 1")
  (`KismetSystemLibrary.ExecuteConsoleCommand` "FoliageQuality 1")
  (`KismetSystemLibrary.ExecuteConsoleCommand` "sg.EffectsQuality 1"))

(event `MainMenustart`
  ;[1 1 1] Main menu
  (`self.Main_menu_show`))

(event `JoinServer`
  (params (SessionToJoin :type "BlueprintSessionResult Structure"))
  ;[1 1 1] Join Server
  (`self.ShowLoadingScreen`)
  (`JoinSessionCallbackProxy.JoinSession` (`GameplayStatics.GetPlayerController` 0) SessionToJoin))

(event `High_Settings`
  ;[1 1 1] Game graphics
  (`KismetSystemLibrary.ExecuteConsoleCommand` "r.ScreenPercentage 100%")
  (`KismetSystemLibrary.ExecuteConsoleCommand` "r.ViewDistanceScale 10000000.0")
  (`KismetSystemLibrary.ExecuteConsoleCommand` "r.PostProcessAAQuality 255555")
  (`KismetSystemLibrary.ExecuteConsoleCommand` "sg.PostProcessQuality 2")
  (`KismetSystemLibrary.ExecuteConsoleCommand` "sg.ShadowQuality 2")
  (`KismetSystemLibrary.ExecuteConsoleCommand` "sg.TextureQuality 2")
  (`KismetSystemLibrary.ExecuteConsoleCommand` "FoliageQuality 2")
  (`KismetSystemLibrary.ExecuteConsoleCommand` "sg.EffectsQuality 2"))

(event `Main_menu_show`
  (bind _returnvalue (`GameplayStatics.GetPlayerController` 0))
  ;[1 1 1] Main menu
  (`/Engine/EditorBlueprintResources/StandardMacros.IsValid` (`self.MainMenuWB`)
    (:`Is Valid`
      _)
    (:`Is Not Valid`
      (bind _returnvalue_2 (`|CreateWidget` "/Game/Pregame/Widgets/Main_menuWB.Main_menuWB_C" _returnvalue))
      (set `self.MainMenuWB` _returnvalue_2)))
  (`UserWidget.AddToViewport` (`self.MainMenuWB`) 0)
  (set `PlayerController.bShowMouseCursor` true _returnvalue))

(event `ShowHostMenu`
  (bind _returnvalue (`GameplayStatics.GetPlayerController` 0))
  ;[1 1 1] Host Game menu
  (`/Engine/EditorBlueprintResources/StandardMacros.IsValid` (`self.HostMenuWB`)
    (:`Is Valid`
      _)
    (:`Is Not Valid`
      (bind _returnvalue_2 (`|CreateWidget` "/Game/Pregame/Widgets/Host_menu.Host_menu_C" _returnvalue))
      (set `self.HostMenuWB` _returnvalue_2)))
  (`UserWidget.AddToViewport` (`self.HostMenuWB`) 0)
  (set `PlayerController.bShowMouseCursor` true _returnvalue))

(event `ShowLoadingScreen`
  ;[1 1 1] Show Loading screen
  (`/Engine/EditorBlueprintResources/StandardMacros.IsValid` (`self.LoadingScreenWB`)
    (:`Is Valid`
      _)
    (:`Is Not Valid`
      (bind _returnvalue (`|CreateWidget` "/Game/Pregame/Widgets/Loading_Screen.Loading_Screen_C" (`GameplayStatics.GetPlayerController` 0)))
      (set `self.LoadingScreenWB` _returnvalue)))
  (`UserWidget.AddToViewport` (`self.LoadingScreenWB`) 0))

(event `ShowServerMenu`
  ;[1 1 1] Server menu Created each time
  (bind _returnvalue (`|CreateWidget` "/Game/Pregame/Widgets/Server_menu.Server_menu_C" (`GameplayStatics.GetPlayerController` 0)))
  (`UserWidget.AddToViewport` _returnvalue 0))

(event `DestroySessionCollar`
  (params (PlayerController :type "PlayerController Object Reference"))
  ;[1 1 1] Destroy Session When Called
  (`DestroySessionCallbackProxy.DestroySession` PlayerController))

(event `Launch Lobby`
  (params (NumberofPlayers :type Integer) (`LAN?` :type Boolean) (ServerName :type Text))
  ;[1 1 1] Launch Lobby
  (set `self.Max Players` NumberofPlayers)
  (set `self.Server Bane` ServerName)
  (`self.ShowLoadingScreen`)
  (`CreateSessionCallbackProxy.CreateSession` (`GameplayStatics.GetPlayerController` 0) (`self.Max Players`) `LAN?`
    (:`OnSuccess`
      (`GameplayStatics.OpenLevel` "Lobby" true "listen"))))

(event `ShowOptionsMenu`
  ;[1 1 1] Show Options Menu
  (`/Engine/EditorBlueprintResources/StandardMacros.IsValid` (`self.OptionsMenuWB`)
    (:`Is Valid`
      _)
    (:`Is Not Valid`
      (bind _returnvalue (`|CreateWidget` "/Game/Pregame/Widgets/Options_menu.Options_menu_C" (`GameplayStatics.GetPlayerController` 0)))
      (set `self.OptionsMenuWB` _returnvalue)))
  (`UserWidget.AddToViewport` (`self.OptionsMenuWB`) 0))

(event `/Game/UltimateStatsComp/Blueprints/Interfaces/BPI_USC_SaveCommunication.SaveActorStatsDataToGameInstance`
  (params (SaveName :type Name) (StatsComponent :type "/Game/UltimateStatsComp/Blueprints/AC_USC_Stats Object Reference"))
  (bind _savedatastruct (`/Game/UltimateStatsComp/Blueprints/AC_USC_Stats.PrepareStatsSaveDataStruct` StatsComponent))
  (`BlueprintMapLibrary.Map_Add` (`self.SavedDataStructs`) SaveName _savedatastruct))

(event `/Game/UltimateStatsComp/Blueprints/Interfaces/BPI_USC_SaveCommunication.LoadActorStatsDataFromGameInstance`
  (params (SaveName :type Name) (StatsComponent :type "/Game/UltimateStatsComp/Blueprints/AC_USC_Stats Object Reference"))
  (bind (_value _returnvalue) (`BlueprintMapLibrary.Map_Find` (`self.SavedDataStructs`) SaveName))
  (if _returnvalue
    (`/Game/UltimateStatsComp/Blueprints/AC_USC_Stats.ReadDataFromStatsDataStruct` StatsComponent _value)))