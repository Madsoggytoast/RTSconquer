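; Demo character for the Ultimate Stats component that handles health, mana, XP, level and periodic effects.
; AnyDamage lowers clamped Health and destroys the actor at zero.
; Effect ticks regenerate Health or Mana, or deal burning and stack-scaled poison damage through ApplyDamage, feeding back into AnyDamage.
; Stat changes reach the controller's HUD through client update events and also call the component's client refresh.
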(event `self.AC_USC_Stats.OnExperienceReceived`
  (params (ExperienceGained :type Integer) (CurrentExperience :type Integer) (NeededExperience :type Integer))
  (`|ExecutionSequence`
    (:`then_0`
      (if (> ExperienceGained 0)
        _))
    (:`then_1`
      (bind _controllerreference (`self.ControllerReference`)
        (:`then`
          (bind _hudreference (`/Game/UltimateStatsComp/DemoData/Blueprints/BP_DemoUSC_PlayerController.HUDReference` _controllerreference)
            (:`then`
              (`TextBlock.SetText` (`/Game/UltimateStatsComp/DemoData/Blueprints/WBP_DemoUSC_CustomCharacterInfoWindow.Text_XP` _hudreference) (`|FormatText` "XP {current}/{needed}" CurrentExperience NeededExperience))
              (`ProgressBar.SetPercent` (`/Game/UltimateStatsComp/DemoData/Blueprints/WBP_DemoUSC_CustomCharacterInfoWindow.ProgressBar_XP` _hudreference) (/ (`KismetMathLibrary.Conv_IntToDouble` CurrentExperience) (`KismetMathLibrary.Conv_IntToDouble` NeededExperience))))
            (:`else`)))
        (:`else`)))))

(event `self.AC_USC_Stats.OnLevelUp`
  (params (LevelReached :type Integer))
  (`self.UpdateLevel_CLIENT` LevelReached))

(event `self.AC_USC_Stats.OnEffectTickExecuted`
  (params (EffectType :type "/Game/UltimateStatsComp/Enumerations/E_USC_EffectType Enum" :default "NewEnumerator0") (EffectStruct :type "/Game/UltimateStatsComp/Structures/S_USC_EffectDynamicData Structure"))
  (switch `/Game/UltimateStatsComp/Enumerations/E_USC_EffectType` EffectType
    (:`NewEnumerator0`
      (`self.Effect_HealthRegeneration` EffectStruct))
    (:`NewEnumerator1`
      (`self.Effect_Burning` EffectStruct))
    (:`NewEnumerator2`
      (`self.Effect_Poisoning` EffectStruct))
    (:`NewEnumerator3`
      (`self.Effect_ManaRegeneration` EffectStruct))))

(event `self.ReceiveAnyDamage`
  (params (Damage :type "Float (single-precision)") (DamageType :type "DamageType Object Reference") (InstigatedBy :type "Controller Object Reference") (DamageCauser :type "Actor Object Reference"))
  (bind _value (`BlueprintMapLibrary.Map_Find` (`/Game/UltimateStatsComp/Blueprints/AC_USC_Stats.CurrentStats` (`self.AC_USC_Stats`)) "NewEnumerator1"))
  (`BlueprintMapLibrary.Map_Add` (`/Game/UltimateStatsComp/Blueprints/AC_USC_Stats.CurrentStats` (`self.AC_USC_Stats`)) "NewEnumerator1" (`KismetMathLibrary.FClamp` (- (`BlueprintMapLibrary.Map_Find` (`/Game/UltimateStatsComp/Blueprints/AC_USC_Stats.CurrentStats` (`self.AC_USC_Stats`)) "NewEnumerator1") Damage) 0.0 (`.FinalValue_9_72CA6EAC410161A8DBACDEA210F24628` (break `/Game/UltimateStatsComp/Structures/S_USC_BaseStat` (`BlueprintMapLibrary.Map_Find` (`/Game/UltimateStatsComp/Blueprints/AC_USC_Stats.BaseStats` (`self.AC_USC_Stats`)) "NewEnumerator1")))))
  (`|ExecutionSequence`
    (:`then_0`
      (`self.UpdateHealthBar_CLIENT` (`BlueprintMapLibrary.Map_Find` (`/Game/UltimateStatsComp/Blueprints/AC_USC_Stats.CurrentStats` (`self.AC_USC_Stats`)) "NewEnumerator1") (`.FinalValue_9_72CA6EAC410161A8DBACDEA210F24628` (break `/Game/UltimateStatsComp/Structures/S_USC_BaseStat` (`BlueprintMapLibrary.Map_Find` (`/Game/UltimateStatsComp/Blueprints/AC_USC_Stats.BaseStats` (`self.AC_USC_Stats`)) "NewEnumerator1")))))
    (:`then_1`
      (`/Game/UltimateStatsComp/Blueprints/AC_USC_Stats.RefreshStatValue_CLIENT` (`self.AC_USC_Stats`) "NewEnumerator1" (`.FinalValue_9_72CA6EAC410161A8DBACDEA210F24628` (break `/Game/UltimateStatsComp/Structures/S_USC_BaseStat` (`BlueprintMapLibrary.Map_Find` (`/Game/UltimateStatsComp/Blueprints/AC_USC_Stats.BaseStats` (`self.AC_USC_Stats`)) "NewEnumerator1"))) _value)
      (if (not (> _value 0.0))
        (`self.OnDeathEvent`)))))

(event `OnDeathEvent`
  (`self.K2_DestroyActor`))

(event `self.AC_USC_Stats.OnBaseStatFinalValueChanged`
  (params (StatType :type "/Game/UltimateStatsComp/Enumerations/E_USC_StatType Enum" :default "NewEnumerator0") (PreviousStatFinalValue :type "Float (single-precision)") (NewStatFinalValue :type "Float (single-precision)") (CurrentStatValue :type "Float (single-precision)"))
  (switch `/Game/UltimateStatsComp/Enumerations/E_USC_StatType` StatType
    (:`NewEnumerator1`
      (`self.UpdateHealthBar_CLIENT` CurrentStatValue NewStatFinalValue))
    (:`NewEnumerator2`
      (`self.UpdateManaBar_CLIENT` CurrentStatValue NewStatFinalValue))))

(event `UpdateHealthBar_CLIENT`
  (params (CurrentHealth :type "Float (double-precision)") (MaximumHealth :type "Float (double-precision)"))
  (bind _controllerreference (`self.ControllerReference`)
    (:`then`
      (bind _hudreference (`/Game/UltimateStatsComp/DemoData/Blueprints/BP_DemoUSC_PlayerController.HUDReference` _controllerreference))
      (`TextBlock.SetText` (`/Game/UltimateStatsComp/DemoData/Blueprints/WBP_DemoUSC_CustomCharacterInfoWindow.Text_HealthCurrent` _hudreference) (`KismetTextLibrary.Conv_DoubleToText` CurrentHealth "HalfToZero" true 1 324 0 0))
      (`TextBlock.SetText` (`/Game/UltimateStatsComp/DemoData/Blueprints/WBP_DemoUSC_CustomCharacterInfoWindow.Text_HealthMax` _hudreference) (`KismetTextLibrary.Conv_DoubleToText` MaximumHealth "HalfToZero" true 1 324 0 0))
      (`ProgressBar.SetPercent` (`/Game/UltimateStatsComp/DemoData/Blueprints/WBP_DemoUSC_CustomCharacterInfoWindow.ProgressBar_Health` _hudreference) (/ CurrentHealth MaximumHealth)))
    (:`else`)))

(event `UpdateManaBar_CLIENT`
  (params (CurrentMana :type "Float (double-precision)") (MaximumMana :type "Float (double-precision)"))
  (bind _controllerreference (`self.ControllerReference`)
    (:`then`
      (bind _hudreference (`/Game/UltimateStatsComp/DemoData/Blueprints/BP_DemoUSC_PlayerController.HUDReference` _controllerreference))
      (`TextBlock.SetText` (`/Game/UltimateStatsComp/DemoData/Blueprints/WBP_DemoUSC_CustomCharacterInfoWindow.Text_ManaCurrent` _hudreference) (`KismetTextLibrary.Conv_DoubleToText` CurrentMana "HalfToZero" true 1 324 0 0))
      (`TextBlock.SetText` (`/Game/UltimateStatsComp/DemoData/Blueprints/WBP_DemoUSC_CustomCharacterInfoWindow.Text_ManaMax` _hudreference) (`KismetTextLibrary.Conv_DoubleToText` MaximumMana "HalfToZero" true 1 324 0 0))
      (`ProgressBar.SetPercent` (`/Game/UltimateStatsComp/DemoData/Blueprints/WBP_DemoUSC_CustomCharacterInfoWindow.ProgressBar_Mana` _hudreference) (/ CurrentMana MaximumMana)))
    (:`else`)))

(event `UpdateLevel_CLIENT`
  (params (LevelReached :type Integer))
  (bind _controllerreference (`self.ControllerReference`)
    (:`then`
      (bind _hudreference (`/Game/UltimateStatsComp/DemoData/Blueprints/BP_DemoUSC_PlayerController.HUDReference` _controllerreference)
        (:`then`
          (`TextBlock.SetText` (`/Game/UltimateStatsComp/DemoData/Blueprints/WBP_DemoUSC_CustomCharacterInfoWindow.Text_Level` _hudreference) (`|FormatText` "Level {value}" LevelReached)))
        (:`else`)))
    (:`else`)))

(fn `Effect_Burning`
  (params (EffectStruct :type "/Game/UltimateStatsComp/Structures/S_USC_EffectDynamicData Structure"))
  (`GameplayStatics.ApplyDamage` self (`.EffectPower_37_A1B05A4B44EACE9CD0F33AA4BE91B94F` (break `/Game/UltimateStatsComp/Structures/S_USC_EffectStaticData` (`.EffectStaticData_22_99A114744E1E5D506A5D9092F9D94929` (break `/Game/UltimateStatsComp/Structures/S_USC_EffectDynamicData` EffectStruct))))))

(fn `Effect_HealthRegeneration`
  (params (EffectStruct :type "/Game/UltimateStatsComp/Structures/S_USC_EffectDynamicData Structure"))
  (bind _currentstats (`/Game/UltimateStatsComp/Blueprints/AC_USC_Stats.CurrentStats` (`self.AC_USC_Stats`)))
  (bind _value (`BlueprintMapLibrary.Map_Find` (`/Game/UltimateStatsComp/Blueprints/AC_USC_Stats.CurrentStats` (`self.AC_USC_Stats`)) "NewEnumerator1"))
  (bind (_basevalue _otherflatbonuses _otherpercentagebonuses _attributeflatbonus _attributepercentagebonus _finalvalue) (break `/Game/UltimateStatsComp/Structures/S_USC_BaseStat` (`BlueprintMapLibrary.Map_Find` (`/Game/UltimateStatsComp/Blueprints/AC_USC_Stats.BaseStats` (`self.AC_USC_Stats`)) "NewEnumerator1")))
  (`BlueprintMapLibrary.Map_Add` _currentstats "NewEnumerator1" (`KismetMathLibrary.FClamp` (+ (`BlueprintMapLibrary.Map_Find` _currentstats "NewEnumerator1") (`.EffectPower_37_A1B05A4B44EACE9CD0F33AA4BE91B94F` (break `/Game/UltimateStatsComp/Structures/S_USC_EffectStaticData` (`.EffectStaticData_22_99A114744E1E5D506A5D9092F9D94929` (break `/Game/UltimateStatsComp/Structures/S_USC_EffectDynamicData` EffectStruct))))) 0.0 (`.FinalValue_9_72CA6EAC410161A8DBACDEA210F24628` (break `/Game/UltimateStatsComp/Structures/S_USC_BaseStat` (`BlueprintMapLibrary.Map_Find` (`/Game/UltimateStatsComp/Blueprints/AC_USC_Stats.BaseStats` (`self.AC_USC_Stats`)) "NewEnumerator1")))))
  (`self.UpdateHealthBar_CLIENT` _value _finalvalue)
  (`/Game/UltimateStatsComp/Blueprints/AC_USC_Stats.RefreshStatValue_CLIENT` (`self.AC_USC_Stats`) "NewEnumerator1" _finalvalue _value))

(fn `Effect_ManaRegeneration`
  (params (EffectStruct :type "/Game/UltimateStatsComp/Structures/S_USC_EffectDynamicData Structure"))
  (bind _currentstats (`/Game/UltimateStatsComp/Blueprints/AC_USC_Stats.CurrentStats` (`self.AC_USC_Stats`)))
  (bind _value (`BlueprintMapLibrary.Map_Find` (`/Game/UltimateStatsComp/Blueprints/AC_USC_Stats.CurrentStats` (`self.AC_USC_Stats`)) "NewEnumerator2"))
  (bind (_basevalue _otherflatbonuses _otherpercentagebonuses _attributeflatbonus _attributepercentagebonus _finalvalue) (break `/Game/UltimateStatsComp/Structures/S_USC_BaseStat` (`BlueprintMapLibrary.Map_Find` (`/Game/UltimateStatsComp/Blueprints/AC_USC_Stats.BaseStats` (`self.AC_USC_Stats`)) "NewEnumerator2")))
  (`BlueprintMapLibrary.Map_Add` _currentstats "NewEnumerator2" (`KismetMathLibrary.FClamp` (+ (`BlueprintMapLibrary.Map_Find` _currentstats "NewEnumerator2") (`.EffectPower_37_A1B05A4B44EACE9CD0F33AA4BE91B94F` (break `/Game/UltimateStatsComp/Structures/S_USC_EffectStaticData` (`.EffectStaticData_22_99A114744E1E5D506A5D9092F9D94929` (break `/Game/UltimateStatsComp/Structures/S_USC_EffectDynamicData` EffectStruct))))) 0.0 (`.FinalValue_9_72CA6EAC410161A8DBACDEA210F24628` (break `/Game/UltimateStatsComp/Structures/S_USC_BaseStat` (`BlueprintMapLibrary.Map_Find` (`/Game/UltimateStatsComp/Blueprints/AC_USC_Stats.BaseStats` (`self.AC_USC_Stats`)) "NewEnumerator2")))))
  (`self.UpdateManaBar_CLIENT` _value _finalvalue)
  (`/Game/UltimateStatsComp/Blueprints/AC_USC_Stats.RefreshStatValue_CLIENT` (`self.AC_USC_Stats`) "NewEnumerator2" _finalvalue _value))

(fn `Effect_Poisoning`
  (params (EffectStruct :type "/Game/UltimateStatsComp/Structures/S_USC_EffectDynamicData Structure"))
  (bind (_stacksamount _ticksleft _timetonearesttick _effectstaticdata) (break `/Game/UltimateStatsComp/Structures/S_USC_EffectDynamicData` EffectStruct))
  (`GameplayStatics.ApplyDamage` self (* _stacksamount (`.EffectPower_37_A1B05A4B44EACE9CD0F33AA4BE91B94F` (break `/Game/UltimateStatsComp/Structures/S_USC_EffectStaticData` _effectstaticdata)))))

(fn `ReplenishHealthAndMana`
  (bind _basestats (`/Game/UltimateStatsComp/Blueprints/AC_USC_Stats.BaseStats` (`self.AC_USC_Stats`)))
  (bind (_basevalue _otherflatbonuses _otherpercentagebonuses _attributeflatbonus _attributepercentagebonus _finalvalue) (break `/Game/UltimateStatsComp/Structures/S_USC_BaseStat` (`BlueprintMapLibrary.Map_Find` _basestats "NewEnumerator2")))
  (bind (_basevalue_2 _otherflatbonuses_2 _otherpercentagebonuses_2 _attributeflatbonus_2 _attributepercentagebonus_2 _finalvalue_2) (break `/Game/UltimateStatsComp/Structures/S_USC_BaseStat` (`BlueprintMapLibrary.Map_Find` _basestats "NewEnumerator1")))
  (`BlueprintMapLibrary.Map_Add` (`/Game/UltimateStatsComp/Blueprints/AC_USC_Stats.CurrentStats` (`self.AC_USC_Stats`)) "NewEnumerator1" _finalvalue_2)
  (`self.UpdateHealthBar_CLIENT` _finalvalue_2 _finalvalue_2)
  (`/Game/UltimateStatsComp/Blueprints/AC_USC_Stats.RefreshStatValue_CLIENT` (`self.AC_USC_Stats`) "NewEnumerator1" _finalvalue_2 _finalvalue_2)
  (`BlueprintMapLibrary.Map_Add` (`/Game/UltimateStatsComp/Blueprints/AC_USC_Stats.CurrentStats` (`self.AC_USC_Stats`)) "NewEnumerator2" _finalvalue)
  (`self.UpdateManaBar_CLIENT` _finalvalue _finalvalue)
  (`/Game/UltimateStatsComp/Blueprints/AC_USC_Stats.RefreshStatValue_CLIENT` (`self.AC_USC_Stats`) "NewEnumerator2" _finalvalue _finalvalue))

(fn `UserConstructionScript`)